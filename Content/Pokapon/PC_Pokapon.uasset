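; PC_Pokapon is the player controller for Pokapon, routing hammer and shield input for two players through a single controller.
; On BeginPlay it adds the IMC_Pokapon Enhanced Input mapping context and caches the BP_PokaponPawn actors tagged Player1 and Player2.
; Separate per-player input actions call PushHammer or PushShield on the matching cached pawn, with no possession involved in the routing.
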(event `self.ReceiveBeginPlay`
  (bind _returnvalue (subsystem `EnhancedInputLocalPlayerSubsystem`))
  (`|ExecutionSequence`
    (:`then_0`
      (`/Engine/EditorBlueprintResources/StandardMacros.IsValid` _returnvalue
        (:`Is Valid`
          (`EnhancedInputSubsystemInterface.AddMappingContext` _returnvalue "/Game/Pokapon/Inputs/IMC_Pokapon.IMC_Pokapon" 0 (struct)))))
    (:`then_1`
      (bind _outactors (`GameplayStatics.GetAllActorsWithTag` "Player1"))
      (bind _asbp_pokapon_pawn (cast `/Game/Pokapon/BP_PokaponPawn` (`|GetArrayItem` _outactors)))
      (set `self.Player1` _asbp_pokapon_pawn))
    (:`then_2`
      (bind _outactors_2 (`GameplayStatics.GetAllActorsWithTag` "Player2"))
      (bind _asbp_pokapon_pawn_2 (cast `/Game/Pokapon/BP_PokaponPawn` (`|GetArrayItem` _outactors_2)))
      (set `self.Player2` _asbp_pokapon_pawn_2))))

(event `EnhancedInput|/Game/Pokapon/Inputs/IA_HammerP1`
  (params (ActionValue :type Boolean) (ElapsedSeconds :type "Float (double-precision)") (TriggeredSeconds :type "Float (double-precision)") (InputAction :type "InputAction Object Reference" :default "/Game/Pokapon/Inputs/IA_HammerP1.IA_HammerP1"))
  ;[1 1 1] Inputs
  (:`Triggered`
    (`/Game/Pokapon/BP_PokaponPawn.Push Hammer` (`self.Player1`))))

(event `EnhancedInput|/Game/Pokapon/Inputs/IA_HammerP2`
  (params (ActionValue :type Boolean) (ElapsedSeconds :type "Float (double-precision)") (TriggeredSeconds :type "Float (double-precision)") (InputAction :type "InputAction Object Reference" :default "/Game/Pokapon/Inputs/IA_HammerP2.IA_HammerP2"))
  ;[1 1 1] Inputs
  (:`Triggered`
    (`/Game/Pokapon/BP_PokaponPawn.Push Hammer` (`self.Player2`))))

(event `EnhancedInput|/Game/Pokapon/Inputs/IA_ShieldP1`
  (params (ActionValue :type Boolean) (ElapsedSeconds :type "Float (double-precision)") (TriggeredSeconds :type "Float (double-precision)") (InputAction :type "InputAction Object Reference" :default "/Game/Pokapon/Inputs/IA_ShieldP1.IA_ShieldP1"))
  ;[1 1 1] Inputs
  (:`Triggered`
    (`/Game/Pokapon/BP_PokaponPawn.Push Shield` (`self.Player1`))))

(event `EnhancedInput|/Game/Pokapon/Inputs/IA_ShieldP2`
  (params (ActionValue :type Boolean) (ElapsedSeconds :type "Float (double-precision)") (TriggeredSeconds :type "Float (double-precision)") (InputAction :type "InputAction Object Reference" :default "/Game/Pokapon/Inputs/IA_ShieldP2.IA_ShieldP2"))
  ;[1 1 1] Inputs
  (:`Triggered`
    (`/Game/Pokapon/BP_PokaponPawn.Push Shield` (`self.Player2`))))

(fn `UserConstructionScript`)